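; Enemy AI pawn that wanders the navmesh and chases the player once it spots them, ending in a level restart.
; From BeginPlay, Aa issues random nearby moves on a delayed loop until PawnSensing sets the Bakıyor flag.
; CustomEvent then runs AI MoveTo on the player; on success it shows the Kokutucu widget and calls RestartLevel after a delay.
; The flag is never cleared after a sighting, so wandering does not resume.
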(event OnSeePawn(PawnSensing)
  (params (Pawn :type Pawn%20Object%20Reference))
  (Variables|Default|Setbakıyor true)
  (CallFunction|CustomEvent))

(event Custom|CustomEvent
  (if (Variables|Default|Getbakıyor)
    (AI|AIMoveTo self "0, 0, 0" (Game|Player|GetPlayerPawn 0) 5.0 false
      (:OnSuccess
        (bind _returnvalue (UserInterface|CreateWidget "/Game/ai/kokutucu.kokutucu_C"))
        (UserInterface|Viewport|AddtoViewport _returnvalue 0)
        (Utilities|FlowControl|Delay 2.0)
        (Development|ExecuteConsoleCommand "RestartLevel " 0)
        (Development|PrintString "Hello")
        (Utilities|FlowControl|Delay 3.0)
        (CallFunction|CustomEvent)))
    (else
      (CallFunction|Aa)
      (Variables|Default|Setbakıyor false))))

(event Custom|aa
  (bind _randomlocation (Class|NavigationSystemV1|GetRandomLocationinNavigableRadius (Transformation|GetActorLocation) 1e+03 0 0))
  (AI|AIMoveTo self _randomlocation 0 5.0 false
    (:then
      (Utilities|FlowControl|Delay 3.0)
      (if (not (Variables|Default|Getbakıyor))
        (CallFunction|Aa)))))

(event EventBeginPlay
  (CallFunction|Aa)
  (Variables|Default|Setbakıyor false))

(fn ConstructionScript)